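; RTS player controller that drives the camera pawn for panning and zooming.
; On BeginPlay it casts player pawn 0 to RTS_CameraPlayer_BP and caches the reference.
; Move axes feed world X and Y input vectors into the pawn's FloatingPawnMovement.
; Zoom actions step the SpringArm's arm length by a zoom speed within clamped limits, and a reset action restores a fixed default length.
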(event EventBeginPlay
  (Utilities|ReferenceCast))

(event Input|ActionEvents|InputActionZoomReset
  (params (Key :type Key%20Structure :default "None"))
  ;[1 1 1] Zoom Controls
  ;;[1 1 1] Reset Zoom
  (:Pressed
    (Variables|/Script/Engine.SpringArmComponent|SetTargetArmLength (Variables|/Game/RTS_Tutorial/Blueprints/RTS_CameraPlayer_BP.RTS_CameraPlayer_BP_C|GetSpringArm (Variables|References|GetCamera%20Pawn%20Ref)) 8e+02)))

(event Input|ActionEvents|InputActionZoomIn
  (params (Key :type Key%20Structure :default "None"))
  (bind _camera_pawn_ref (Variables|References|GetCamera%20Pawn%20Ref))
  (bind _springarm (Variables|/Game/RTS_Tutorial/Blueprints/RTS_CameraPlayer_BP.RTS_CameraPlayer_BP_C|GetSpringArm _camera_pawn_ref))
  ;[1 1 1] Zoom Controls
  ;;[1 1 1] Zoom In
  (:Pressed
    (Variables|/Script/Engine.SpringArmComponent|SetTargetArmLength _springarm (Math|Float|Clamp(Float) (- (Variables|/Script/Engine.SpringArmComponent|GetTargetArmLength _springarm) (Variables|MovementVariables|GetZoomSpeed)) (Variables|MovementVariables|GetMinZoomLimit) (Variables|MovementVariables|GetMaxZoomLimit)))))

(event Input|ActionEvents|InputActionZoomOut
  (params (Key :type Key%20Structure :default "None"))
  (bind _camera_pawn_ref (Variables|References|GetCamera%20Pawn%20Ref))
  (bind _springarm (Variables|/Game/RTS_Tutorial/Blueprints/RTS_CameraPlayer_BP.RTS_CameraPlayer_BP_C|GetSpringArm _camera_pawn_ref))
  ;[1 1 1] Zoom Controls
  ;;[1 1 1] Zoom Out
  (:Pressed
    (Variables|/Script/Engine.SpringArmComponent|SetTargetArmLength _springarm (Math|Float|Clamp(Float) (+ (Variables|MovementVariables|GetZoomSpeed) (Variables|/Script/Engine.SpringArmComponent|GetTargetArmLength _springarm)) (Variables|MovementVariables|GetMinZoomLimit) (Variables|MovementVariables|GetMaxZoomLimit)))))

(event Input|AxisEvents|InputAxisMoveForward
  (params (AxisValue :type Float%20%28single-precision%29))
  (Class|PawnMovementComponent|AddInputVector (Variables|/Game/RTS_Tutorial/Blueprints/RTS_CameraPlayer_BP.RTS_CameraPlayer_BP_C|GetFloatingPawnMovement (Variables|References|GetCamera%20Pawn%20Ref)) (Math|Vector|MakeVector AxisValue 0.0 0.0) false))

(event Input|AxisEvents|InputAxisMoveRight
  (params (AxisValue :type Float%20%28single-precision%29))
  (Class|PawnMovementComponent|AddInputVector (Variables|/Game/RTS_Tutorial/Blueprints/RTS_CameraPlayer_BP.RTS_CameraPlayer_BP_C|GetFloatingPawnMovement (Variables|References|GetCamera%20Pawn%20Ref)) (Math|Vector|MakeVector 0.0 AxisValue 0.0) false))

(fn ConstructionScript)